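; BP_Lift03 is a lift with swinging double doors that makes a one-way ride upward.
; A collision volume opens and closes the doors through a timeline, with opening blocked while the lift moves.
; Interacting with Box closes the doors and runs the slowed MoveLift timeline to raise the platform, reopening them on arrival.
; A second volume sets MoveReady, which nothing here reads.
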(event OnComponentBeginOverlap(MoveCollision)
  (params (OverlappedComponent :type Primitive%20Component%20Object%20Reference) (OtherActor :type Actor%20Object%20Reference) (OtherComp :type Primitive%20Component%20Object%20Reference) (OtherBodyIndex :type Integer) (bFromSweep :type Boolean) (SweepResult :type Hit%20Result%20Structure%20%28by%20ref%29))
  (Variables|Default|SetMoveReady true))

(event OnComponentEndOverlap(Collision)
  (params (OverlappedComponent :type Primitive%20Component%20Object%20Reference) (OtherActor :type Actor%20Object%20Reference) (OtherComp :type Primitive%20Component%20Object%20Reference) (OtherBodyIndex :type Integer))
  ;[1 1 1] AutoOpenAndColseDoor
  (bind _newtrack_0 (Timeline|Timeline Reverse)
    (:Update
      (Transformation|SetRelativeRotation (Variables|Default|GetLift02Door01) (Math|Rotator|MakeRotator 0.0 0.0 (* (* _newtrack_0 3e+01) -1.0)) false false)
      (Transformation|SetRelativeRotation (Variables|Default|GetLift02Door02) (Math|Rotator|MakeRotator 0.0 0.0 (* _newtrack_0 3e+01)) false false))))

(event OnComponentBeginOverlap(Collision)
  (params (OverlappedComponent :type Primitive%20Component%20Object%20Reference) (OtherActor :type Actor%20Object%20Reference) (OtherComp :type Primitive%20Component%20Object%20Reference) (OtherBodyIndex :type Integer) (bFromSweep :type Boolean) (SweepResult :type Hit%20Result%20Structure%20%28by%20ref%29))
  ;[1 1 1] AutoOpenAndColseDoor
  (if (not (Variables|Default|GetMove))
    (bind _newtrack_0 (Timeline|Timeline Play)
      (:Update
        (Transformation|SetRelativeRotation (Variables|Default|GetLift02Door01) (Math|Rotator|MakeRotator 0.0 0.0 (* (* _newtrack_0 3e+01) -1.0)) false false)
        (Transformation|SetRelativeRotation (Variables|Default|GetLift02Door02) (Math|Rotator|MakeRotator 0.0 0.0 (* _newtrack_0 3e+01)) false false)))))

(event EventProcessInteraction
  (params (NewParam :type Scene%20Component%20Object%20Reference))
  ;[1 1 1] AutoOpenAndColseDoor
  (if (== NewParam (Variables|Default|GetBox))
    (Utilities|FlowControl|Sequence
      (:then_0
        (bind _newtrack_0 (Timeline|Timeline Reverse)
          (:Update
            (Transformation|SetRelativeRotation (Variables|Default|GetLift02Door01) (Math|Rotator|MakeRotator 0.0 0.0 (* (* _newtrack_0 3e+01) -1.0)) false false)
            (Transformation|SetRelativeRotation (Variables|Default|GetLift02Door02) (Math|Rotator|MakeRotator 0.0 0.0 (* _newtrack_0 3e+01)) false false))))
      (:then_1
        (Variables|Default|SetMove true)
        (bind _newtrack_0_2 (Timeline|MoveLift Play)
          (:Update
            (Transformation|SetRelativeLocation (Variables|Default|GetLift02) (Math|Vector|MakeVector 0.0 0.0 (Math|Float|Lerp -3e+03 0.0 _newtrack_0_2)) false false))
          (:Finished
            (Variables|Default|SetMove false)
            (Timeline|Timeline Play)))))))

(event EventBeginPlay
  (Components|Timeline|SetPlayRate (Variables|Default|GetMoveLift) (/ 1.0 5.0)))

(fn ConstructionScript)